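; BP_NPC is an NPC Blueprint with a projectile attack and a hide-when-detected visibility behavior.
; Invisibility hides the mesh and its children when IsDetected and starts a timer with no event bound; otherwise it shows the mesh alone.
; CheckInvisibility randomly triggers UpdateVisibility, which runs Invisibility, while Attack spawns BP_Projectile.
; BeginPlay only sets IsVisible if undetected; calls to Attack and the visibility check are unwired.
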(event `self.ReceiveBeginPlay`
  (if (not (`self.IsDetected?`))
    (set `self.IsVisible` true)))

(event `UpdateVisibility`
  ;[0 0 0 0.5] Visibilité
  (`self.Invisibility`))

(event `CheckInvisibility`
  ;[0 0 0 0.5] Visibilité
  (if (`KismetMathLibrary.RandomBool`)
    (`self.UpdateVisibility`)))

(fn `Attack`
  (`|SpawnActorFromClass` "/Game/Blueprint/BP_Projectile.BP_Projectile_C" (`self.Spawn Transform`) "Undefined" "MultiplyWithRoot" null null)
  (return))

(fn `Invisibility`
  (if (`self.IsDetected?`)
    (`KismetSystemLibrary.K2_SetTimerDelegate` :`Time` 5.0)
    (`SceneComponent.SetVisibility` (`self.Mesh`) false true)
    (else
      (`SceneComponent.SetVisibility` (`self.Mesh`) true false))))

(fn `UserConstructionScript`)